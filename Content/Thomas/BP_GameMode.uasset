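; Game mode that runs a timed round, tracking score, a blaster charge and the game-over sequence.
; BeginPlay shows the HUD and resets timer and charge, while a Delay on Tick drives the one-second countdown.
; Scoring adds points, and BlasterCount builds charge until firing is allowed at the maximum.
; At zero time, GameOver explodes the player with radial damage, shows the end screen and cursor, then pauses after a short delay.
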(event `self.ReceiveBeginPlay`
  ;[1 1 1] Start Parameter
  (bind _returnvalue (`|CreateWidget` "/Game/Thomas/UI/PlayerInterface.PlayerInterface_C"))
  (`UserWidget.AddToViewport` _returnvalue 0)
  (set `self.TimeSec` 120)
  (set `self.BlasterCounts` 0.0)
  (set `self.MaxBlasterCounts` (`self.MaxBlasterCounts`))
  (set `self.canFireBlaster` false))

(event `self.ReceiveTick`
  (params (DeltaSeconds :type "Float (single-precision)"))
  ;[1 1 1] Timer
  (`KismetSystemLibrary.Delay` 1.0)
  (set `self.TimeSec` (- (`self.TimeSec`) 1))
  (if (<= (`self.TimeSec`) 0)
    (set `self.TimeSec` 0)
    (`self.GameOver`)))

(event `Scoring`
  (params (AdditionalScore :type Integer))
  ;[1 1 1] Score
  (set `self.ScorePoints` (+ AdditionalScore (`self.ScorePoints`))))

(event `BlasterCount`
  ;[1 1 1] Secondary
  (if (>= (`self.BlasterCounts`) (`self.MaxBlasterCounts`))
    (set `self.BlasterCounts` (`self.MaxBlasterCounts`))
    (set `self.canFireBlaster` true)
    (else
      (set `self.BlasterCounts` (+ (`self.BlasterCounts`) 1.0))
      (set `self.canFireBlaster` false))))

(event `GameOver`
  ;[1 1 1] End Game
  (bind _asbp_player (cast `/Game/Thomas/BP_Player` (`GameplayStatics.GetPlayerCharacter` 0)))
  (`CharacterMovementComponent.DisableMovement` (`Character.CharacterMovement` _asbp_player))
  (`|SpawnActorFromClass` "/Game/Thomas/Explosion.Explosion_C" (`KismetMathLibrary.MakeTransform` (`self.K2_GetActorLocation` _asbp_player) (struct) (5.0 5.0 5.0)) "Undefined" "OverrideRootScale" null null)
  (`GameplayStatics.ApplyRadialDamage` :`BaseDamage` (`self.Base Damage Amount`) :`Origin` (`SceneComponent.K2_GetComponentLocation` (`Character.CapsuleComponent` _asbp_player)) :`DamageRadius` 1500.0 :`DamageCauser` (`self.GetInstigator` _asbp_player) :`InstigatedByController` (`self.GetInstigatorController` _asbp_player))
  (bind _returnvalue (`|CreateWidget` "/Game/Thomas/UI/GameOver.GameOver_C"))
  (`UserWidget.AddToViewport` _returnvalue 0)
  (set `PlayerController.bShowMouseCursor` true (`GameplayStatics.GetPlayerController` 0))
  (`self.K2_DestroyActor` _asbp_player)
  (`KismetSystemLibrary.Delay` 0.5)
  (`GameplayStatics.SetGamePaused` true))

(fn `UserConstructionScript`)